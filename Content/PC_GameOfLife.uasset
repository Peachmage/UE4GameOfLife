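; Player controller for a Game of Life game that shows the mouse cursor and lets the player paint cells on the grid.
; While the Drawing axis is held, a cursor trace finds the grid instance under the mouse and sets that cell active, or inactive with Left Shift held.
; Edits apply only while the simulation is inactive.
; The last hit instance is cached to avoid re-toggling the same cell until the cursor moves or input releases.
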(event EventBeginPlay
  (Variables|Default|SetbShowMouseCursor true))

(event EventTick
  (params (DeltaSeconds :type Float%20%28single-precision%29)))

(event Input|AxisEvents|InputAxisDrawing
  (params (AxisValue :type Float%20%28single-precision%29))
  (bind (_hitresult _returnvalue) (Game|Player|GetHitResultUnderCursorbyChannel "TraceTypeQuery1" true))
  (bind (_bblockinghit _binitialoverlap _time _distance _location _impactpoint _normal _impactnormal _physmat _hitactor _hitcomponent _hitbonename _hititem) (Collision|BreakHitResult _hitresult))
  (if (> AxisValue 0.0)
    (if _returnvalue
      (if (!= _hititem (Variables|Default|GetLastSquareHit))
        (bind _asgame_of_life_actor (Utilities|Casting|CastToGameOfLifeActor _hitactor))
        (if (and (== (Variables|/Script/ConvaysLife.GameOfLifeActor|GetGrid _asgame_of_life_actor) _hitcomponent) (not (Class|GameOfLifeActor|IsGameActive _asgame_of_life_actor)))
          (Variables|Default|SetLastSquareHit _hititem)
          (Class|GameOfLifeActor|ToggleCell _asgame_of_life_actor (Class|GameOfLifeActor|GetCellfromInstanceID _asgame_of_life_actor _hititem) (not (Game|Player|IsInputKeyDown "LeftShift"))))))
    (else
      (Variables|Default|SetLastSquareHit -2))))

(fn ConstructionScript)